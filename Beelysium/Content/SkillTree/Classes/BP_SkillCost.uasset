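; BP_SkillCost defines an XP cost for unlocking a skill in the skill tree.
; CanUnlockSkill checks that the player's SkillTreeXP on BP_ThirdPersonCharacter covers SkillTreeXPNeeded, returning false if the cast fails.
; ApplyUnlockCost subtracts that amount from the character's XP without rechecking the balance.
; GetUnlockText builds the "XP Required" label through string conversion.
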(fn ApplyUnlockCost
  (params (Player :type Pawn%20Object%20Reference))
  (bind _asbp_third_person_character (Utilities|Casting|CastToBP_ThirdPersonCharacter Player))
  (Variables|/Game/ThirdPerson/Blueprints/BP_ThirdPersonCharacter.BP_ThirdPersonCharacter_C|SetSkillTreeXP _asbp_third_person_character (- (Variables|/Game/ThirdPerson/Blueprints/BP_ThirdPersonCharacter.BP_ThirdPersonCharacter_C|GetSkillTreeXP _asbp_third_person_character) (Variables|Default|GetSkillTreeXPNeeded))))

(fn CanUnlockSkill
  (params (Player :type Pawn%20Object%20Reference))
  (bind _asbp_third_person_character (Utilities|Casting|CastToBP_ThirdPersonCharacter Player)
    (:then
      (return (>= (Variables|/Game/ThirdPerson/Blueprints/BP_ThirdPersonCharacter.BP_ThirdPersonCharacter_C|GetSkillTreeXP _asbp_third_person_character) (Variables|Default|GetSkillTreeXPNeeded))))
    (:CastFailed
      (return false))))

(fn GetUnlockText
  (params (Player :type Pawn%20Object%20Reference))
  (return (Utilities|Text|ToText(String) (Utilities|String|Append (Utilities|String|ToString(Text) (Utilities|Text|MakeLiteralText "XP Required : ")) (Utilities|String|ToString(Integer) (Variables|Default|GetSkillTreeXPNeeded))))))